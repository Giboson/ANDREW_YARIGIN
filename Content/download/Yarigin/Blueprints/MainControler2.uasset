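; MainControler2 is a player controller that manages the HUD, game-over state and respawn for the MainCharacter.
; On BeginPlay it creates the MainUIX and Menu widgets and caches the controlled pawn.
; Each tick it pushes health and lamp or weapon interaction text to MainUIX, and toggles the game-over screen, cursor and input mode as health crosses zero.
; Restart spawns and possesses a new character at the first PlayerStart found.
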(event Custom|Restart
  ;[1 1 1] Restart
  (bind _outactors (Actor|GetAllActorsOfClass "/Script/Engine.PlayerStart"))
  (bind _returnvalue (Game|SpawnActorfromClass "/Game/download/Yarigin/Blueprints/MainCharacter.MainCharacter_C" (Transformation|GetActorTransform (Utilities|Array|Get(acopy) _outactors)) "AlwaysSpawn" 0 0))
  (Variables|Default|SetMyPawen _returnvalue)
  (Pawn|UnPossess)
  (Pawn|Possess (Variables|Default|GetMyPawen)))

(event EventTick
  (params (DeltaSeconds :type Float%20%28single-precision%29))
  (bind _mypawen (Variables|Default|GetMyPawen))
  (bind _mypawen_2 (Variables|Default|GetMyPawen))
  (bind _statusac (Variables|/Game/download/Yarigin/Blueprints/MainCharacter.MainCharacter_C|GetStatusAC _mypawen_2))
  (bind _activewepon (Variables|/Game/download/Yarigin/Blueprints/MainCharacter.MainCharacter_C|GetActiveWepon _mypawen))
  (Utilities|FlowControl|Sequence
    (:then_0
      (|CollapseGraph_0
        (:execute
          (Development|PrintString "MainConroler2" true true "(R=0.046242,G=1.000000,B=0.000000,A=1.000000)" 0.0))))
    (:then_1
      ;[1 1 1] Informaiton level Health
      (Default|UpdateHealth (Variables|Default|GetMainWidjet) (Variables|/Game/download/Yarigin/Blueprints/StatusAC.StatusAC_C|GetHealth _statusac) (Variables|/Game/download/Yarigin/Blueprints/StatusAC.StatusAC_C|GetMaxHeallh _statusac))
      (Default|Update|Interact (Variables|Default|GetMainWidjet)))
    (:then_2
      ;[1 1 1] Revers else
      (Utilities|FlowControl|Sequence
        (:then_0
          ;[1 1 1] information text Lamp [E]
          (if (Utilities|IsValid (Variables|/Game/download/Yarigin/Blueprints/MainCharacter.MainCharacter_C|GetAs%20Beas%20Lamp (Variables|Default|GetMyPawen)))
            (Default|Update|Interact (Variables|Default|GetMainWidjet) "Activate")
            (else
              (Default|Update|Interact (Variables|Default|GetMainWidjet)))))
        (:then_1
          (if (Utilities|IsValid _activewepon)
            ;[1 1 1] information text gun [E]
            (Default|Update|Interact (Variables|Default|GetMainWidjet) (Utilities|String|ToString(Name) (Variables|/Game/download/Yarigin/Meshes/WeaponBeas.WeaponBeas_C|GetName _activewepon)))))))
    (:then_3
      (if (Variables|Default|GetPlayerAlive)
        (if (<= (Variables|/Game/download/Yarigin/Blueprints/StatusAC.StatusAC_C|GetHealth (Variables|/Game/download/Yarigin/Blueprints/MainCharacter.MainCharacter_C|GetStatusAC (Variables|Default|GetMyPawen))) 0.0)
          (Variables|Default|SetPlayerAlive false)
          (Default|SwitchScreen (Variables|Default|GetMainWidjet) 1)
          (Variables|Default|SetbShowMouseCursor true)
          (Default|PlayGameOverAnimation (Variables|Default|GetMainWidjet))
          (Input|SetInputModeUIOnly self (Variables|Default|GetMainWidjet) "DoNotLock"))
        (elif (> (Variables|/Game/download/Yarigin/Blueprints/StatusAC.StatusAC_C|GetHealth (Variables|/Game/download/Yarigin/Blueprints/MainCharacter.MainCharacter_C|GetStatusAC (Variables|Default|GetMyPawen))) 0.0)
          (Variables|Default|SetPlayerAlive true)
          (Default|SwitchScreen (Variables|Default|GetMainWidjet))
          (Variables|Default|SetbShowMouseCursor false)
          (Input|SetInputModeGameOnly self))))))

(event EventBeginPlay
  (Utilities|FlowControl|Sequence
    (:then_0
      (bind _returnvalue (UserInterface|CreateWidget "/Game/download/Yarigin/Characters/Minimap/Intersfes/MainUIX.MainUIX_C"))
      (Variables|Default|SetMainWidjet _returnvalue)
      (UserInterface|Viewport|AddtoViewport (Variables|Default|GetMainWidjet) 0))
    (:then_1
      ;[1 1 1] Informaiton user
      (bind _asmain_character (Utilities|Casting|CastToMainCharacter (Pawn|GetControlledPawn)))
      (Variables|Default|SetMyPawen _asmain_character))
    (:then_2
      (bind _returnvalue_2 (UserInterface|CreateWidget "/Game/download/Yarigin/Characters/Minimap/Intersfes/Menu.Menu_C"))
      (UserInterface|Viewport|AddtoViewport _returnvalue_2 0))))

(fn ConstructionScript)