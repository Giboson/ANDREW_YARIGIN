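; StatusAC is a character component combining health (damage, healing, death callback) with a parkour system for wall runs, vertical wall runs, ledge grabs and mantles.
; Initialize caches the character and starts a looping ~60 Hz timer driving gated movement updates and camera roll.
; Traces detect walls and ledges, LaunchCharacter propels runs, and interpolation performs mantles.
; A parkour mode enum coordinates transitions; Tick prints health and calls the run-ending functions.
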(event Custom|Initialize
  (params (Character :type Character%20Object%20Reference))
  ;[1 1 1] Jump user
  (bind _output_get (Variables|Default|SetCharacter Character))
  (bind _output_get_2 (Variables|Default|SetCharacter%20Movement (Variables|/Script/Engine.Character|GetCharacterMovement _output_get)))
  ;[1 1 1] Time Jamp users
  (Variables|Default|SetDefault%20Gravity%20Scale (Variables|/Script/Engine.CharacterMovementComponent|GetGravityScale _output_get_2))
  (Utilities|Time|SetTimerbyEvent (delegate Custom|WallRunUpdateEvent) 0.0167 true))

(event Custom|JumpEvent
  (if (Utilities|Enum|Equal(Enum) (Variables|Default|GetPrev%20ParkourMovementMode) "NewEnumerator0")
    (if (AI|Components|NavMovement|IsFalling (Variables|Default|GetCharacter%20Movement))
      (CallFunction|OpenGates)
      (CallFunction|PlayCameraShake "/Game/download/Yarigin/Blueprints/CameraSakes/JumpLand.JumpLand_C"))))

(event Custom|Land%20Event)

(event Custom|WallRunUpdateEvent
  (Utilities|FlowControl|Sequence
    (:then_0
      (|WallRun))
    (:then_1
      (|OpenWallRunGate))
    (:then_2
      (|Mantie))
    (:then_3
      (CallFunction|CameraTick))))

(event Custom|ResetWallRunSuppression)

(event Custom|MovementCanged
  (params (PrevParkourMovementMode :type E_ParkurMovementType%20Enum :default "NewEnumerator0") (New%20ParkourMode :type E_ParkurMovementType%20Enum :default "NewEnumerator0"))
  (Variables|Default|SetPrev%20ParkourMovementMode PrevParkourMovementMode)
  (Variables|Default|SetCurrent%20ParkourMovementMode New%20ParkourMode)
  (CallFunction|RestaMovement))

(event Custom|ParkourMovemetChanged
  (params (Prev%20MovementMode :type EMovementMode%20Enum :default "MOVE_None") (New%20MovementMode :type EMovementMode%20Enum :default "MOVE_None"))
  (Utilities|IsValid (Variables|Default|GetCharacter%20Movement)
    (:Is%20Valid
      (Variables|Default|SetPrevMovementMode Prev%20MovementMode)
      (Variables|Default|SetCurrentMovementMode New%20MovementMode)
      (|OpenGateNode))))

(event Custom|PlayCameraShake
  (params (Shake :type Camera%20Shake%20Base%20Class%20Reference))
  (if (Variables|Default|GetCameraShake)
    (Camera|PlayWorldCameraShake Shake (Transformation|GetActorLocation (Variables|Default|GetCharacter)) 0.0 1e+02)))

(event EventTick
  (params (DeltaSeconds :type Float%20%28single-precision%29))
  (Utilities|FlowControl|Sequence
    (:then_0
      ;[1 1 1] Damage Logic
      (Development|PrintString (Utilities|String|ToString(Float) (Variables|Default|GetHealth)) true true "(R=0.073642,G=1.000000,B=0.000000,A=1.000000)" DeltaSeconds))
    (:then_1
      (CallFunction|WallRunEnd 0.0)
      (CallFunction|VerticalWallRunEnd 0.0)
      (CallFunction|CloseGates)
      (CallFunction|PlayCameraShake "/Game/download/Yarigin/Blueprints/CameraSakes/JumpLand.JumpLand_C"))))

(event EventBeginPlay
  ;[1 1 1] Damage Logic
  (Variables|Default|SetHealth (Variables|Default|GetMaxHeallh)))

(fn Damege
  (params (Damege :type Float%20%28single-precision%29))
  (Variables|Default|SetHealth (Math|Float|Clamp(Float) (Math|Float|Max(Float) (- (Variables|Default|GetHealth) Damege) 0.0) 0.0 (Variables|Default|GetMaxHeallh)))
  (if (<= (Variables|Default|GetHealth) 0.0)
    (Default|CallOnDeath)))

(fn IsDead
  (return (<= (Variables|Default|GetHealth) 0.0)))

(fn AddHeatlh
  (params (Add :type Float%20%28single-precision%29))
  (Variables|Default|SetHealth (Math|Float|Min(Float) (+ Add (Variables|Default|GetHealth)) (Variables|Default|GetMaxHeallh))))

(fn GetHeatlh
  (return (Variables|Default|GetHealth)))

(fn Recovery
  (Variables|Default|SetHealth (Variables|Default|GetMaxHeallh)))

(fn WallRunUpdate
  (if (Utilities|WallRunning?)
    (bind _onwall (CallFunction|WallRunMovemint (Transformation|GetActorLocation (Variables|Default|GetCharacter)) (.Right (Utilities|WallRunEndVectors)) -1.0)) ; Right
    (if _onwall
      (CallFunction|SetParkourMovementMode "NewEnumerator2")
      (CallFunction|OpenWallRunGate? :!label _label)
      (elif (Utilities|Enum|Equal(Enum) (Variables|Default|GetPrev%20ParkourMovementMode) "NewEnumerator2")
        (CallFunction|WallRunEnd 1.0)
        (else
          (CallFunction|WallRunMovemint (Transformation|GetActorLocation (Variables|Default|GetCharacter)) (.left (Utilities|WallRunEndVectors)) 1.0) ; Right
          (if true
            (CallFunction|SetParkourMovementMode "NewEnumerator1")
            (goto _label)
            (else
              (CallFunction|WallRunEnd 0.5))))))
    (else
      (CallFunction|WallRunEnd 1.0))))

(fn WallRunMovemint
  (params (Start :type Vector) (End :type Vector) (WallRunDirection :type Float%20%28single-precision%29))
  (bind _outhit (Collision|LineTraceByChannel Start End "TraceTypeQuery1" false 0 "None"))
  (if (.bblockinghit _outhit)
    (if (and (AI|Components|NavMovement|IsFalling (Variables|Default|GetCharacter%20Movement)) (.ReturnValue (Utilities|ValidWallRunVector? (.normal _outhit))))
      (Variables|Default|SetWallRunNormal (.InVce2 (Utilities|ValidWallRunVector? (.normal _outhit))))
      (Character|LaunchCharacter (Variables|Default|GetCharacter) (* (Math|Vector|CrossProduct (Variables|Default|GetWallRunNormal) "0, 0,1.000000") (* (Variables|Default|GetWallRunSpeed) WallRunDirection)) true (not (Variables|Default|GetWallRunGraviy))) ; Move Forward
      (return true)
      (else
        (return false)))
    (else
      (return false))))

(fn WallRunEnd
  (params (Rest%20Time :type Float%20%28single-precision%29))
  (if (Utilities|WallRunning?)
    (bind _change (CallFunction|SetParkourMovementMode "NewEnumerator0"))
    (if _change
      (Utilities|Time|SetTimerbyFunctionName 0 "OpenWallRunGate" Rest%20Time))))

(fn SuppressWallRun
  (params (Delay :type Float%20%28single-precision%29))
  (Variables|Default|SetWallRunSeppressed? true)
  (Utilities|Time|SetTimerbyFunctionName 0 "ResetWallRunSuppression" Delay))

(fn CameraTick
  (switch Utilities|FlowControl|Switch|SwitchonE_ParkurMovementType (Variables|Default|GetCurrent%20ParkourMovementMode)
    (:NewEnumerator0
      (CallFunction|CameraTilt 0.0 :!label _label))
    (:NewEnumerator1
      (CallFunction|CameraTilt 15.0))
    (:NewEnumerator2
      (CallFunction|CameraTilt -15.0 :!label _label_2))
    (:NewEnumerator3
      (goto _label))
    (:NewEnumerator4
      (goto _label))
    (:NewEnumerator5
      (goto _label))
    (:NewEnumerator6
      (goto _label_2))
    (:NewEnumerator7
      (goto _label))))

(fn CameraTilt
  (params (Target%20X%20%28Roll%29 :type Float%20%28single-precision%29))
  (bind _character (Variables|Default|GetCharacter))
  (bind _returnvalue (Pawn|GetController _character))
  (bind _returnvalue_2 (Pawn|GetControlRotation _returnvalue :!class /Script/Engine.Controller))
  (bind (_roll _pitch _yaw) (Math|Rotator|BreakRotator _returnvalue_2))
  (Pawn|SetControlRotation (Pawn|GetController (Variables|Default|GetCharacter)) (Math|Interpolation|RInterpTo _returnvalue_2 (Math|Rotator|MakeRotator Target%20X%20%28Roll%29 _pitch _yaw) 0.0 0.0)))

(fn WallRunJump
  (bind _wallrunnormal (Variables|Default|GetWallRunNormal))
  (bind _wallrunjumpoffforce (Variables|Default|GetWallRunJumpOffForce))
  (if (Utilities|WallRunning?)
    (CallFunction|WallRunEnd 0.35)
    (Character|LaunchCharacter (Variables|Default|GetCharacter) (Math|Vector|MakeVector (* _wallrunjumpoffforce (.x _wallrunnormal)) (* _wallrunjumpoffforce (.y _wallrunnormal)) (Variables|Default|GetWallRunJumpHeitght)) false true)))

(fn RestaMovement
  (if (Utilities|Enum|Equal(Enum) (Variables|Default|GetCurrent%20ParkourMovementMode) "NewEnumerator0")
    (Variables|/Script/Engine.CharacterMovementComponent|SetGravityScale (Variables|Default|GetCharacter%20Movement) (Variables|Default|GetDefault%20Gravity%20Scale))
    (Pawn|Components|CharacterMovement|SetMovementMode (Variables|Default|GetCharacter%20Movement) (Utilities|Select :Index (Variables|Default|GetPrev%20ParkourMovementMode) :NewEnumerator0 "MOVE_Falling" :NewEnumerator1 "MOVE_Falling" :NewEnumerator2 "MOVE_Falling" :NewEnumerator3 "MOVE_Falling" :NewEnumerator4 "MOVE_Falling" :NewEnumerator5 "MOVE_Walking" :NewEnumerator6 "MOVE_Walking" :NewEnumerator7 "MOVE_Walking") 0)))

(fn SetParkourMovementMode
  (params (NewMode :type E_ParkurMovementType%20Enum :default "NewEnumerator0"))
  (if (Utilities|Enum|Equal(Enum) NewMode (Variables|Default|GetCurrent%20ParkourMovementMode))
    (return false)
    (else
      (CallFunction|ParkourMovemetChanged (Variables|Default|GetPrevMovementMode) (Variables|Default|GetCurrentMovementMode))
      (return true))))

(fn OpenWallRunGate?
  (Variables|/Script/Engine.CharacterMovementComponent|SetGravityScale (Variables|Default|GetCharacter%20Movement) (Math|Interpolation|FInterpTo (Variables|/Script/Engine.CharacterMovementComponent|GetGravityScale (Variables|Default|GetCharacter%20Movement)) (Variables|Default|GetWallRunTrageGravity) (Utilities|Time|GetWorldDeltaSeconds) 1e+01)))

(fn VerticalWallRunUpdate
  (bind (_eyes _feet) (Utilities|MantleVectors))
  (if (Utilities|CanVectcalWallRun)
    (bind (_outhit _returnvalue) (Collision|CapsuleTraceByChannel _eyes _feet 2e+01 1e+01 "TraceTypeQuery1" false 0 "None"))
    (if _returnvalue
      (Variables|Default|SetMantieTraceDistance (.Distance (Collision|BreakHitResult _outhit)))
      (if (Class|CharacterMovementComponent|IsWalkable (Variables|Default|GetCharacter%20Movement) _outhit)
        (Variables|Default|SetMantlePosition (+ (.ImpactPoint (Collision|BreakHitResult _outhit)) (Math|Vector|MakeVector 0.0 0.0 (Variables|/Script/Engine.CapsuleComponent|GetCapsuleHalfHeight (Variables|/Script/Engine.Character|GetCapsuleComponent (Variables|Default|GetCharacter))))))
        (CallFunction|CloseVectcalWallRunGate)
        (|LedgeGrab)
        (if (Utilities|QuitMantle)
          (CallFunction|OpenMantieChekGate)
          (else
            (Utilities|Time|SetTimerbyFunctionName 0 "OpenMantleCheckGrate" 0.25)))
        (else
          (CallFunction|VerticalWallRunMovement :!label _label)))
      (else
        (goto _label)))
    (else
      (CallFunction|VerticalWallRunEnd 0.35))))

(fn VerticalWallRunEnd
  (params (RestartTime :type Float%20%28single-precision%29))
  (bind _current_parkourmovementmode (Variables|Default|GetCurrent%20ParkourMovementMode))
  (if (Math|Boolean|ORBoolean (Utilities|Enum|Equal(Enum) _current_parkourmovementmode "NewEnumerator4") (Utilities|Enum|Equal(Enum) _current_parkourmovementmode "NewEnumerator3") (Utilities|Enum|Equal(Enum) _current_parkourmovementmode "NewEnumerator5"))
    (bind _change (CallFunction|SetParkourMovementMode "NewEnumerator0"))
    (if _change
      (CallFunction|CloseVectcalWallRunGate)
      (CallFunction|ClouseMantieChekGate)
      (Utilities|Time|SetTimerbyFunctionName 0 "OpenVericalWallRunGate" RestartTime))))

(fn VerticalWallRunMovement
  (bind _feet (Utilities|MantleVectors))
  (bind (_outhit _returnvalue) (Collision|LineTraceByChannel _feet (+ _feet (* (Transformation|GetActorForwardVector (Variables|Default|GetCharacter)) 5e+01)) "TraceTypeQuery1" false 0 "None"))
  (if (and (> (Utilities|ForwardInput) 0.0) _returnvalue)
    (Variables|Default|SetVerticalWallRunNormal (.ImpactNormal (Collision|BreakHitResult _outhit)))
    (CallFunction|SetParkourMovementMode "NewEnumerator3")
    (Character|LaunchCharacter (Variables|Default|GetCharacter) (Math|Vector|MakeVector (.x (* (Variables|Default|GetVerticalWallRunNormal) -6e+02)) (.y (* (Variables|Default|GetVerticalWallRunNormal) -6e+02)) (Variables|Default|GetVerticalWallRunSpeed)) true true)
    (else
      (CallFunction|VerticalWallRunEnd 0.35))))

(fn MantleMovement
  (bind _character (Variables|Default|GetCharacter))
  (bind _character_2 (Variables|Default|GetCharacter))
  (bind _wallrunnormal (Variables|Default|GetWallRunNormal))
  (bind _returnvalue (Pawn|GetController _character_2))
  (bind _returnvalue_2 (Transformation|GetActorLocation _character))
  (Pawn|SetControlRotation _returnvalue (Math|Interpolation|RInterpTo (Pawn|GetControlRotation _returnvalue :!class /Script/Engine.Controller) (Math|Rotator|FindLookatRotation (Math|Vector|MakeVector (.x _returnvalue_2) (.y _returnvalue_2) 0.0) (Math|Vector|MakeVector (.x _wallrunnormal) (.y _wallrunnormal) 0.0)) (Utilities|Time|GetWorldDeltaSeconds) 7.0))
  (Transformation|SetActorLocation (Variables|Default|GetCharacter) (Math|Interpolation|VInterpTo (Transformation|GetActorLocation (Variables|Default|GetCharacter)) (Variables|Default|GetMantlePosition) (Utilities|Time|GetWorldDeltaSeconds) (select (Utilities|QuitMantle) (Variables|Default|GetQuikMantleSeed) (Variables|Default|GetMantleSpeed))) false false)
  (if (< (Math|Vector|Distance(Vector) (Transformation|GetActorLocation (Variables|Default|GetCharacter)) (Variables|Default|GetMantlePosition)) 8.0)
    (CallFunction|VerticalWallRunEnd 0.5)))

(fn OpenGates
  (CallFunction|OpenWallRunGate?)
  (CallFunction|OpenVericalWallRunGate))

(fn CloseGates
  (CallFunction|OpenWallRunGate?)
  (CallFunction|CloseVectcalWallRunGate))

(event Custom|ClouseMantieChekGate
  (Utilities|FlowControl|Gate true) ; enters at Close
)

(event Custom|OpenMantieChekGate
  (Utilities|FlowControl|Gate true) ; enters at Open
)

(event Custom|OpenMantieGate
  (Utilities|FlowControl|Gate true) ; enters at Open
)

(event Custom|CloseMantieGate
  (Utilities|FlowControl|Gate true) ; enters at Close
)

(event Custom|MantieChek
  (if (Utilities|CanMantle)
    (CallFunction|MantieStart)))

(event Custom|MantieStart
  (bind _change (CallFunction|SetParkourMovementMode "NewEnumerator5"))
  (if _change
    (CallFunction|PlayCameraShake (select (Utilities|QuitMantle) "/Game/download/Yarigin/Blueprints/CameraSakes/QuickMante.QuickMante_C" "/Game/download/Yarigin/Blueprints/CameraSakes/Mante.Mante_C"))
    (CallFunction|ClouseMantieChekGate)
    (CallFunction|OpenMantieGate)))

(event Custom|OpenVericalWallRunGate
  (Utilities|FlowControl|Gate true) ; enters at Open
)

(event Custom|CloseVectcalWallRunGate
  (CallFunction|CloseMantieGate)
  (Utilities|FlowControl|Gate true) ; enters at Close
)